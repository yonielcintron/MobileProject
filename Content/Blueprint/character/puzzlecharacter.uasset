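; Puzzle character Blueprint that can jump on input and display an animated selection cursor.
; Enable and disable functions cast the SelectionCursor component's widget to selectionlcon, then toggle the component's visibility along with an endlessly looping cursor animation.
; The cursor is disabled on BeginPlay, and nothing in this Blueprint calls the enable function.
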(event EventBeginPlay
  (CallFunction|DisableSelectionWidget))

(event Collision|EventActorBeginOverlap
  (params (OtherActor :type Actor%20Object%20Reference)))

(event EventTick
  (params (DeltaSeconds :type Float%20%28single-precision%29)))

(event Input|ActionEvents|InputActionjump
  (params (Key :type Key%20Structure :default "None"))
  (:Pressed
    (Character|Jump)))

(fn ConstructionScript)

(fn EnableSelectionWidget
  (bind _selectioncursor (Variables|Default|GetSelectionCursor))
  (bind _asselectionlcon (Utilities|Casting|CastToselectionlcon (UserInterface|GetUserWidgetObject _selectioncursor)))
  (UserInterface|Animation|PlayAnimation _asselectionlcon (Variables|/Game/hud/selectionlcon.selectionlcon_C|GetcursorAnimation _asselectionlcon) 0.0 0 "Forward" 1.0 false)
  (Rendering|SetVisibility _selectioncursor true false))

(fn DisableSelectionWidget
  (bind _selectioncursor (Variables|Default|GetSelectionCursor))
  (bind _asselectionlcon (Utilities|Casting|CastToselectionlcon (UserInterface|GetUserWidgetObject _selectioncursor)))
  (Class|UserWidget|StopAnimation _asselectionlcon (Variables|/Game/hud/selectionlcon.selectionlcon_C|GetcursorAnimation _asselectionlcon))
  (Rendering|SetVisibility _selectioncursor false false))