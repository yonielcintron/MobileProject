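; Player controller for a touch-driven puzzle game with selectable characters viewed through per-character camera volumes.
; A short tap selects, switches or deselects a PuzzleCharacter, possessing it on selection, or sends the selected one to the tapped point.
; Dragging rotates the current volume's camera each Tick, while presses and moves toggle its spline use.
; Character switches preserve or reset camera transforms; the SetDestination click-to-move gate is never entered.
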(event EventBeginPlay
  (Variables|Default|SetbShowMouseCursor true)
  (bind _aspuzzle_character (Utilities|Casting|CastToPuzzleCharacter (Game|Player|GetPlayerPawn 0)))
  (bind _output_get (Variables|Default|SetCurrentCameraVolume (Variables|/Game/Blueprint/character/puzzlecharacter.PuzzleCharacter_C|GetCurrentCameraVolume _aspuzzle_character)))
  (Game|Player|SetViewTargetwithBlend _output_get 0.0 "VTBlend_Linear" 0.0 false))

(event EventTick
  (params (DeltaSeconds :type Float%20%28single-precision%29))
  (bind (_locationx _locationy) (Class|PlayerController|GetInputTouchState "Touch1"))
  (bind (_camera _returnvalue) (CallFunction|Addtocamerarotation))
  (if (Variables|Default|GetFingerPressed)
    (Variables|Default|SetDeltaTime DeltaSeconds)
    (Variables|Default|SetCurrentTouchLocation (Math|Vector2D|MakeVector2D _locationx _locationy))
    (if (and (== (.X (Math|Vector2D|BreakVector2D (Variables|Default|GetPreviousTouchLocation))) -1.0) (== (.Y (Math|Vector2D|BreakVector2D (Variables|Default|GetPreviousTouchLocation))) -1.0))
      (Variables|Default|SetPreviousTouchLocation (Variables|Default|GetCurrentTouchLocation))
      (else
        (Variables|Default|SetDeltaTouchLocation (- (Variables|Default|GetCurrentTouchLocation) (Variables|Default|GetPreviousTouchLocation)))
        (Transformation|SetWorldRotation _camera _returnvalue false false)
        (Variables|Default|SetPreviousTouchLocation (Variables|Default|GetCurrentTouchLocation))))))

(event Input|ActionEvents|InputActionSetDestination
  (params (Key :type Key%20Structure :default "None"))
  (:Pressed
    (Utilities|FlowControl|Gate true) ; enters at Open
  )
  (:Released
    (Utilities|FlowControl|Gate true) ; enters at Close
  ))

(event Input|TouchEvents|InputTouch
  (params (Location :type Vector) (FingerIndex :type ETouchIndex%20Enum))
  (bind _returnvalue (Utilities|Enum|Equal(Enum) FingerIndex "Touch1"))
  (:Pressed
    (if _returnvalue
      (CallFunction|Touchpressed)))
  (:Released
    (if _returnvalue
      (CallFunction|Touchreleased))))

(fn ConstructionScript)

(fn MovetoHitLocation
  (params (Hit :type Vector%20%28by%20ref%29))
  (if (>= (Math|Vector|VectorLength (- (Transformation|GetActorLocation (Game|Player|GetPlayerPawn 0)) Hit)) (Variables|Default|GetMinClickDistance))
    (AI|Navigation|SimpleMovetoLocation self Hit)))

(fn Touchpressed
  (bind _hitresult (Class|PlayerController|GetHitResultUnderFingerbyChannel "Touch1" "TraceTypeQuery1" true))
  (bind (_locationx _locationy) (Class|PlayerController|GetInputTouchState "Touch1"))
  (bind (_bblockinghit _binitialoverlap _time _distance _location _impactpoint _normal _impactnormal _physmat _hitactor) (Collision|BreakHitResult _hitresult))
  (Variables|Default|SetFingerPressed true)
  (Variables|Default|SetInitialTouchLocation (Math|Vector2D|MakeVector2D _locationx _locationy))
  (Variables|Default|SetHit%20Actor _hitactor)
  (Variables|Default|SetHitLocation _location)
  (Utilities|Casting|CastToPuzzleCharacter _hitactor
    (:CastFailed
      (Variables|/Game/Blueprint/cameravolume.CameraVolume_C|SetUseSpline (Variables|Default|GetCurrentCameraVolume) false))))

(fn Touchreleased
  (bind (_locationx _locationy) (Class|PlayerController|GetInputTouchState "Touch1"))
  (bind _hit_actor (Variables|Default|GetHit%20Actor))
  (Variables|Default|SetPreviousTouchLocation "(X=-1.000000,Y=-1.000000)")
  (Variables|Default|SetFingerPressed false)
  (bind _output_get (Variables|Default|SetFinalTouchLocation (Math|Vector2D|MakeVector2D _locationx _locationy)))
  (if (< (Math|Vector2D|Vector2DLength (- (Variables|Default|GetInitialTouchLocation) _output_get)) (Variables|Default|GetMinDragThreshHold))
    (Utilities|IsValid _hit_actor
      (:Is%20Valid
        (bind _aspuzzle_character (Utilities|Casting|CastToPuzzleCharacter _hit_actor)
          (:then
            (Variables|Default|SetHitCharacter _aspuzzle_character)
            ;[1 0 0] Already Have Character Selected?
            (Utilities|IsValid (Variables|Default|GetSelectedCharacter)
              (:Is%20Valid
                (if (!= (Variables|Default|GetHitCharacter) (Variables|Default|GetSelectedCharacter))
                  (CallFunction|ChangeSelectedCharacter)
                  (else
                    ;[1 1 1] un-select the selected character
                    (Default|DisableSelectionWidget (Variables|Default|GetSelectedCharacter))
                    (Variables|Default|SetSelectedCharacter 0))))
              (:Is%20Not%20Valid
                ;[1 1 1] select the character
                (Variables|Default|SetSelectedCharacter (Variables|Default|GetHitCharacter))
                (Variables|/Game/Blueprint/cameravolume.CameraVolume_C|SetCharacter (Variables|/Game/Blueprint/character/puzzlecharacter.PuzzleCharacter_C|GetCurrentCameraVolume (Variables|Default|GetSelectedCharacter)) (Variables|Default|GetSelectedCharacter))
                (Variables|Default|SetCurrentCameraVolume (Variables|/Game/Blueprint/character/puzzlecharacter.PuzzleCharacter_C|GetCurrentCameraVolume (Variables|Default|GetSelectedCharacter)))
                (Default|EnableSelectionWidget (Variables|Default|GetSelectedCharacter))
                (Pawn|Possess (Variables|Default|GetSelectedCharacter))
                (Game|Player|SetViewTargetwithBlend (Variables|/Game/Blueprint/character/puzzlecharacter.PuzzleCharacter_C|GetCurrentCameraVolume (Variables|Default|GetSelectedCharacter)) 0.0 "VTBlend_Linear" 0.0 false))))
          (:CastFailed
            ;[1 1 1] Check if Selected Character. If so, Move
            (Utilities|IsValid (Variables|Default|GetSelectedCharacter)
              (:Is%20Valid
                (CallFunction|MovetoHitLocation (Variables|Default|GetHitLocation))
                (if (Variables|/Game/Blueprint/cameravolume.CameraVolume_C|GetTurnUseSplineBackOn (Variables|Default|GetCurrentCameraVolume))
                  (Variables|/Game/Blueprint/cameravolume.CameraVolume_C|SetUseSpline (Variables|Default|GetCurrentCameraVolume) true))))))))))

(fn Addtocamerarotation
  (bind _currentcameravolume (Variables|Default|GetCurrentCameraVolume))
  (bind _deltatouchlocation (Variables|Default|GetDeltaTouchLocation))
  (bind _swipespeed (Variables|Default|GetSwipeSpeed))
  (bind (_x _y) (Math|Vector2D|BreakVector2D _deltatouchlocation))
  (bind _camera (Variables|/Game/Blueprint/cameravolume.CameraVolume_C|GetCamera _currentcameravolume))
  (bind _returnvalue (Transformation|GetWorldRotation _camera))
  (bind (_roll _pitch _yaw) (Math|Rotator|BreakRotator _returnvalue))
  (return _camera (Math|Interpolation|RInterpTo _returnvalue (Math|Rotator|MakeRotator _roll (* (+ _pitch (* _y -1.0)) _swipespeed) (* (+ _yaw _x) _swipespeed)) (Variables|Default|GetDeltaTime) 2.0)))

(fn ChangeSelectedCharacter
  (if (== (Variables|/Game/Blueprint/character/puzzlecharacter.PuzzleCharacter_C|GetCurrentCameraVolume (Variables|Default|GetHitCharacter)) (Variables|/Game/Blueprint/character/puzzlecharacter.PuzzleCharacter_C|GetCurrentCameraVolume (Variables|Default|GetSelectedCharacter)))
    (LocalVariables|SetPreviousCameraTransform (Transformation|GetWorldTransform (Variables|/Game/Blueprint/cameravolume.CameraVolume_C|GetCamera (Variables|/Game/Blueprint/character/puzzlecharacter.PuzzleCharacter_C|GetCurrentCameraVolume (Variables|Default|GetSelectedCharacter)))))
    (LocalVariables|SetUsePreviousCameraTransform true)
    (else
      (LocalVariables|SetUsePreviousCameraTransform false)))
  (Variables|Default|SetPreviousCameraVolume (Variables|/Game/Blueprint/character/puzzlecharacter.PuzzleCharacter_C|GetCurrentCameraVolume (Variables|Default|GetSelectedCharacter)))
  ;[1 1 1] Un-Select the Selected Character
  (Default|DisableSelectionWidget (Variables|Default|GetSelectedCharacter))
  (Pawn|UnPossess)
  (bind _output_get (Variables|Default|SetSelectedCharacter (Variables|Default|GetHitCharacter)))
  (Default|EnableSelectionWidget _output_get)
  (Pawn|Possess (Variables|Default|GetSelectedCharacter))
  (Variables|/Game/Blueprint/cameravolume.CameraVolume_C|SetCharacter (Variables|/Game/Blueprint/character/puzzlecharacter.PuzzleCharacter_C|GetCurrentCameraVolume (Variables|Default|GetSelectedCharacter)) (Variables|Default|GetSelectedCharacter))
  (Variables|Default|SetCurrentCameraVolume (Variables|/Game/Blueprint/character/puzzlecharacter.PuzzleCharacter_C|GetCurrentCameraVolume (Variables|Default|GetSelectedCharacter)))
  (Game|Player|SetViewTargetwithBlend (Variables|/Game/Blueprint/character/puzzlecharacter.PuzzleCharacter_C|GetCurrentCameraVolume (Variables|Default|GetSelectedCharacter)) 0.0 "VTBlend_Linear" 0.0 false)
  (Utilities|IsValid (Variables|Default|GetPreviousCameraVolume)
    (:Is%20Valid
      (if (LocalVariables|GetUsePreviousCameraTransform)
        (Transformation|SetWorldTransform (Variables|/Game/Blueprint/cameravolume.CameraVolume_C|GetCamera (Variables|Default|GetPreviousCameraVolume)) (LocalVariables|GetPreviousCameraTransform) false false)
        (Variables|Default|SetPreviousCameraVolume 0)
        (if (Variables|/Game/Blueprint/cameravolume.CameraVolume_C|GetTurnUseSplineBackOn (Variables|Default|GetCurrentCameraVolume))
          (Variables|/Game/Blueprint/cameravolume.CameraVolume_C|SetUseSpline (Variables|Default|GetCurrentCameraVolume) true))
        (else
          (Transformation|SetWorldTransform (Variables|/Game/Blueprint/cameravolume.CameraVolume_C|GetCamera (Variables|Default|GetPreviousCameraVolume)) (Variables|/Game/Blueprint/cameravolume.CameraVolume_C|GetInitialCameraTransfrom (Variables|Default|GetPreviousCameraVolume)) false false)
          (Variables|Default|SetPreviousCameraVolume 0)
          (if (Variables|/Game/Blueprint/cameravolume.CameraVolume_C|GetTurnUseSplineBackOn (Variables|Default|GetCurrentCameraVolume))
            (Variables|/Game/Blueprint/cameravolume.CameraVolume_C|SetUseSpline (Variables|Default|GetCurrentCameraVolume) true)))))))