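; PlainsWallDoor is a door that rises vertically when enough switches are active.
; Activate and Deactivate events adjust a switch counter, and reaching SwitchRequirement plays a 2D sound and runs a timeline.
; The timeline adds its DoorElevation track to the mesh's starting Z, cached on BeginPlay.
; Once the count drops below the requirement, the timeline reverses only if StayOpen is false and no switches remain active.
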(event EventBeginPlay
  (Variables|Default|SetInitialDoorLocation (Transformation|GetWorldLocation (Variables|Default|GetdoorMesh))))

(event Collision|EventActorBeginOverlap
  (params (OtherActor :type Actor%20Object%20Reference)))

(event EventTick
  (params (DeltaSeconds :type Float%20%28single-precision%29)))

(event EventActivate
  (bind _initialdoorlocation (Variables|Default|GetInitialDoorLocation))
  (bind (_x _y _z) (Math|Vector|BreakVector _initialdoorlocation))
  (Math|Integer|IncrementInt (Variables|Default|GetSwitchesActivated)
    (:%20%20
      (if (>= (Variables|Default|GetSwitchesActivated) (Variables|Default|GetSwitchRequirement))
        (Audio|PlaySound2D (Variables|Default|GetDoorSound) 1.0 1.0 0.0 0 0)
        (bind _doorelevation (Timeline|doorTimeline Play)
          (:Update
            (Transformation|SetWorldLocation (Variables|Default|GetdoorMesh) (Math|Vector|MakeVector _x _y (+ _doorelevation _z)) false false)))))))

(event EventDeactivate
  (bind _initialdoorlocation (Variables|Default|GetInitialDoorLocation))
  (bind (_x _y _z) (Math|Vector|BreakVector _initialdoorlocation))
  (Math|Integer|DecrementInt (Variables|Default|GetSwitchesActivated)
    (:%20%20
      (if (< (Variables|Default|GetSwitchesActivated) (Variables|Default|GetSwitchRequirement))
        (if (not (or (Variables|Default|GetStayOpen) (> (Variables|Default|GetSwitchesActivated) 0)))
          (bind _doorelevation (Timeline|doorTimeline Reverse)
            (:Update
              (Transformation|SetWorldLocation (Variables|Default|GetdoorMesh) (Math|Vector|MakeVector _x _y (+ _doorelevation _z)) false false))))))))

(fn ConstructionScript)

(fn NewFunction0)