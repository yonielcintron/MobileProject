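; Puzzle game player controller for selecting characters and moving them by touch.
; A touch tap on a character toggles selection widgets, possesses it and blends view to its camera volume; tapping elsewhere sends it there via SimpleMoveToLocation.
; Drag threshold separates taps from drags, and touch press also runs release logic immediately.
; Mouse click-to-move and swipe camera rotation are unfinished, with key execution paths left unconnected.
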(event EventBeginPlay
  (Variables|Default|SetbShowMouseCursor true)
  (bind _aspuzzlecharacter (Utilities|Casting|CastTopuzzlecharacter (Game|Player|GetPlayerPawn 0)))
  (Variables|Default|Setcuirrenntcameravolume (Variables|/Game/Blueprint/character/puzzlecharacter.puzzlecharacter_C|Getcurrentcameravolume _aspuzzlecharacter)))

(event EventTick
  (params (DeltaSeconds :type Float%20%28single-precision%29))
  (bind (_locationx _locationy) (Class|PlayerController|GetInputTouchState "Touch1"))
  (Variables|Default|SetDelta%20time DeltaSeconds)
  (Variables|Default|SetcurrentTouch%20location (Math|Vector2D|MakeVector2D _locationx _locationy))
  (if (and (== (.X (Math|Vector2D|BreakVector2D (Variables|Default|GetpreviousTouch%20location))) -1.0) (== (.Y (Math|Vector2D|BreakVector2D (Variables|Default|GetpreviousTouch%20location))) -1.0))
    (Variables|Default|SetpreviousTouch%20location (Variables|Default|GetcurrentTouch%20location))))

(event Input|ActionEvents|InputActionSetDestination
  (params (Key :type Key%20Structure :default "None"))
  (:Pressed
    (Utilities|FlowControl|Gate true) ; enters at Open
  )
  (:Released
    (Utilities|FlowControl|Gate true) ; enters at Close
  ))

(event Input|TouchEvents|InputTouch
  (params (Location :type Vector) (FingerIndex :type ETouchIndex%20Enum))
  (bind _returnvalue (Utilities|Enum|Equal(Enum) FingerIndex "Touch1"))
  (:Pressed
    (if _returnvalue
      (CallFunction|Touchpressed)
      (CallFunction|Touchreleased (Variables|Default|Getmindragthreshold) :!label _label)))
  (:Released
    (if _returnvalue
      (goto _label))))

(fn ConstructionScript)

(fn MoveTohitLocation
  (params (Hit :type Vector%20%28by%20ref%29))
  (if (>= (Math|Vector|VectorLength (- (Transformation|GetActorLocation (Game|Player|GetPlayerPawn 0)) Hit)) (Variables|Default|Getminclickdistance))
    (AI|Navigation|SimpleMovetoLocation self Hit)))

(fn Touchpressed
  (bind _hitresult (Class|PlayerController|GetHitResultUnderFingerbyChannel "Touch1" "TraceTypeQuery1" true))
  (bind (_locationx _locationy) (Class|PlayerController|GetInputTouchState "Touch1"))
  (bind (_bblockinghit _binitialoverlap _time _distance _location _impactpoint _normal _impactnormal _physmat _hitactor) (Collision|BreakHitResult _hitresult))
  (Variables|Default|Setfingerpressed true)
  (Variables|Default|Setlnitialtouchlocation (Math|Vector2D|MakeVector2D _locationx _locationy))
  (Variables|Default|SetHit%20Actor _hitactor)
  (Variables|Default|SethitLocation _location)
  (Utilities|Casting|CastTopuzzlecharacter _hitactor
    (:CastFailed
      (Variables|/Game/Blueprint/cameravolume.cameravolume_C|Setusespline (Variables|Default|Getcuirrenntcameravolume) false))))

(fn Touchreleased
  (params (B :type Float%20%28single-precision%29) (Object :type Object%20Object%20Reference))
  (bind (_locationx _locationy) (Class|PlayerController|GetInputTouchState "Touch1"))
  (bind _hit_actor (Variables|Default|GetHit%20Actor))
  (bind _cuirrenntcameravolume (Variables|Default|Getcuirrenntcameravolume))
  (Variables|Default|SetpreviousTouch%20location "(X=-1.000000,Y=-1.000000)")
  (Variables|Default|Setfingerpressed false)
  (bind _output_get (Variables|Default|Setfinaltouchlocation (Math|Vector2D|MakeVector2D _locationx _locationy)))
  (if (< (Math|Vector2D|Vector2DLength (- _output_get (Variables|Default|Getlnitialtouchlocation))) (Variables|Default|Getmindragthreshold))
    (Utilities|IsValid _hit_actor
      (:Is%20Valid
        (bind _aspuzzlecharacter (Utilities|Casting|CastTopuzzlecharacter _hit_actor)
          (:then
            (Development|PrintString (Utilities|GetObjectName _aspuzzlecharacter))
            (Variables|Default|Sethitcharacter _aspuzzlecharacter)
            ;[1 0 0] already have character selected?
            (Utilities|IsValid (Variables|Default|Getselectedcharacter)
              (:Is%20Valid
                (if (!= (Variables|Default|Gethitcharacter) (Variables|Default|Getselectedcharacter))
                  ;[1 1 1] un-select the selected character
                  (Default|Disableselectionwidget (Variables|Default|Getselectedcharacter))
                  (Pawn|UnPossess)
                  (bind _output_get_2 (Variables|Default|Setselectedcharacter (Variables|Default|Gethitcharacter)))
                  (Default|Enableselectionwidet _output_get_2)
                  (Pawn|Possess (Variables|Default|Getselectedcharacter))
                  (Game|Player|SetViewTargetwithBlend (Variables|/Game/Blueprint/character/puzzlecharacter.puzzlecharacter_C|Getcurrentcameravolume _output_get_2) 0.0 "VTBlend_Linear" 0.0 false)))
              (:Is%20Not%20Valid
                (bind _output_get_3 (Variables|Default|Setselectedcharacter (Variables|Default|Gethitcharacter)))
                (Default|Enableselectionwidet _output_get_3)
                (Pawn|Possess _output_get_3)
                (Game|Player|SetViewTargetwithBlend (Variables|/Game/Blueprint/character/puzzlecharacter.puzzlecharacter_C|Getcurrentcameravolume _output_get_3) 0.0 "VTBlend_Linear" 0.0 false))))
          (:CastFailed
            (Utilities|IsValid (Variables|Default|Getselectedcharacter)
              (:Is%20Valid
                (CallFunction|MoveTohitLocation (Variables|Default|GethitLocation))
                (if (Variables|/Game/Blueprint/cameravolume.cameravolume_C|Getturnusesplinebackon _cuirrenntcameravolume)
                  (Variables|/Game/Blueprint/cameravolume.cameravolume_C|Setusespline _cuirrenntcameravolume true))))))))))

(fn Addtocamerarotation
  (return 0 (Math|Interpolation|RInterpTo (Transformation|GetWorldRotation (Variables|/Game/Blueprint/cameravolume.cameravolume_C|GetCamera (Variables|Default|Getcuirrenntcameravolume))) "0, 0, 0" 0.0 0.0)))