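; Camera volume actor that takes over the player's view when the puzzle character enters its box.
; On overlap it registers itself as the current camera volume on the character and player controller, then eases the view target to itself.
; With spline mode on, Tick moves the camera to the spline point closest to the character and aims it at them.
; BeginPlay saves the initial spline flag and camera transform, both unused here.
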(event OnComponentBeginOverlap(Box)
  (params (OverlappedComponent :type Primitive%20Component%20Object%20Reference) (OtherActor :type Actor%20Object%20Reference) (OtherComp :type Primitive%20Component%20Object%20Reference) (OtherBodyIndex :type Integer) (bFromSweep :type Boolean) (SweepResult :type Hit%20Result%20Structure%20%28by%20ref%29))
  (bind _aspuzzlecharacter (Utilities|Casting|CastTopuzzlecharacter OtherActor))
  (bind _output_get (Variables|Default|Setcharacter _aspuzzlecharacter))
  (Variables|/Game/Blueprint/character/puzzlecharacter.puzzlecharacter_C|Setcurrentcameravolume _output_get self)
  (Utilities|IsValid (Variables|Default|Getcontroller)
    (:Is%20Valid
      (bind _aspuzzleplayercontorller (Utilities|Casting|CastTopuzzleplayercontorller (Variables|Default|Getcontroller)))
      (Variables|/Game/Blueprint/puzzleplayercontorller.puzzleplayercontorller_C|Setcuirrenntcameravolume _aspuzzleplayercontorller self)
      (Game|Player|SetViewTargetwithBlend (Variables|Default|Getcontroller) self 2.0 "VTBlend_EaseInOut" 5.0 true))))

(event EventBeginPlay
  (Variables|Default|Setcontroller (Game|GetPlayerController 0))
  (Variables|Default|Setturnusesplinebackon (Variables|splinesetting|Getusespline))
  (Variables|Default|Setlnitialcameratransform (Transformation|GetWorldTransform (Variables|Default|GetCamera))))

(event Collision|EventActorBeginOverlap
  (params (OtherActor :type Actor%20Object%20Reference)))

(event EventTick
  (params (DeltaSeconds :type Float%20%28single-precision%29))
  (bind _character (Variables|Default|Getcharacter))
  (bind _capsulecomponent (Variables|/Script/Engine.Character|GetCapsuleComponent _character))
  (bind _returnvalue (Transformation|GetWorldLocation _capsulecomponent))
  (if (Variables|splinesetting|Getusespline)
    (Utilities|IsValid (Variables|Default|Getcharacter)
      (:Is%20Valid
        (Transformation|SetWorldLocationAndRotation (Variables|Default|GetCamera) (Spline|FindLocationClosesttoWorldLocation (Variables|splinesetting|GetSpline) _returnvalue "World") (Math|Rotator|FindLookatRotation (Transformation|GetWorldLocation (Variables|Default|GetCamera)) _returnvalue) false false)))))

(fn ConstructionScript)