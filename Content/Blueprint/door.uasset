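; Door actor that raises its mesh vertically when activated.
; BeginPlay caches the mesh's starting world location, and the Activate event plays a timeline whose DoorElevation track is added to the starting Z each update.
; The graph contains no close or reverse logic, and overlap and tick events are unused.
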(event EventBeginPlay
  (Variables|Default|SetInitialDoorLocation (Transformation|GetWorldLocation (Variables|Default|GetdoorMesh))))

(event Collision|EventActorBeginOverlap
  (params (OtherActor :type Actor%20Object%20Reference)))

(event EventTick
  (params (DeltaSeconds :type Float%20%28single-precision%29)))

(event EventActivate
  (bind _initialdoorlocation (Variables|Default|GetInitialDoorLocation))
  (bind (_x _y _z) (Math|Vector|BreakVector _initialdoorlocation))
  (bind _doorelevation (Timeline|doorTimeline Play)
    (:Update
      (Transformation|SetWorldLocation (Variables|Default|GetdoorMesh) (Math|Vector|MakeVector _x _y (+ _doorelevation _z)) false false))))

(fn ConstructionScript)