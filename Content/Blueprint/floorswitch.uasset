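; Floor switch for a puzzle game that signals linked actors when a PuzzleCharacter steps on or off it.
; Box overlap begin and end send Activate and Deactivate messages to entries in Affectedactors, gated by interface checks.
; A timeline offsets the switch mesh's height from its starting location on step-on.
; Stepping off reverses the timeline inside the actor loop, only for entries passing the check, whose interface is unset there.
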(event OnComponentBeginOverlap(Box)
  (params (OverlappedComponent :type Primitive%20Component%20Object%20Reference) (OtherActor :type Actor%20Object%20Reference) (OtherComp :type Primitive%20Component%20Object%20Reference) (OtherBodyIndex :type Integer) (bFromSweep :type Boolean) (SweepResult :type Hit%20Result%20Structure%20%28by%20ref%29))
  (bind _initialswitchlocation (Variables|Default|Getinitialswitchlocation))
  (bind (_x _y _z) (Math|Vector|BreakVector _initialswitchlocation))
  (Utilities|Casting|CastToPuzzleCharacter OtherActor)
  (for _array_element (Variables|Default|Getaffectedactors)
    (if (Utilities|DoesObjectImplementInterface _array_element "/Game/Blueprint/SwitchInterface.SwitchInterface_C")
      (Class|SwitchInterface|Activate(Message) _array_element)))
  (bind _switcelevation (Timeline|switchtimeline Play)
    (:Update
      (Transformation|SetWorldLocation (Variables|Default|GetSwitchMesh) (Math|Vector|MakeVector _x _y (+ _switcelevation _z)) false false))))

(event OnComponentEndOverlap(Box)
  (params (OverlappedComponent :type Primitive%20Component%20Object%20Reference) (OtherActor :type Actor%20Object%20Reference) (OtherComp :type Primitive%20Component%20Object%20Reference) (OtherBodyIndex :type Integer))
  (bind _initialswitchlocation (Variables|Default|Getinitialswitchlocation))
  (bind (_x _y _z) (Math|Vector|BreakVector _initialswitchlocation))
  ;[1 1 1] send deactivate message if player step off the switch
  (Utilities|Casting|CastToPuzzleCharacter OtherActor)
  (for _array_element (Variables|Default|Getaffectedactors)
    (if (Utilities|DoesObjectImplementInterface _array_element 0)
      (Class|SwitchInterface|Deactivate(Message) _array_element)
      (bind _switcelevation (Timeline|switchtimeline Reverse)
        (:Update
          (Transformation|SetWorldLocation (Variables|Default|GetSwitchMesh) (Math|Vector|MakeVector _x _y (+ _switcelevation _z)) false false))))))

(event EventBeginPlay
  (Variables|Default|Setinitialswitchlocation (Transformation|GetWorldLocation (Variables|Default|GetSwitchMesh))))

(fn ConstructionScript)